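; BP_ProjectileCinematic is a projectile actor that pushes physics objects it strikes, apparently intended for cinematics.
; On BeginPlay it starts a one-shot timer that destroys it after TimeToLive.
; On a hit, it applies an impulse at its own location to physics-simulating components, using its velocity scaled by MaxImpulse.
; It is not destroyed on impact, only when the timer expires.
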(event Custom|OnTTLExpired
  (Actor|DestroyActor))

(event EventBeginPlay
  (Utilities|Time|SetTimerbyEvent (delegate Custom|OnTTLExpired) (Variables|Default|GetTimeToLive)))

(event Collision|EventHit
  (params (MyComp :type Primitive%20Component%20Object%20Reference) (Other :type Actor%20Object%20Reference) (OtherComp :type Primitive%20Component%20Object%20Reference) (bSelfMoved :type Boolean) (HitLocation :type Vector :default "0, 0, 0") (HitNormal :type Vector :default "0, 0, 0") (NormalImpulse :type Vector :default "0, 0, 0") (Hit :type Hit%20Result%20Structure%20%28by%20ref%29))
  (if (Physics|IsSimulatingPhysics OtherComp "None")
    (Physics|AddImpulseatLocation OtherComp (* (Transformation|GetVelocity) (Variables|Default|GetMax%20Impulse)) (Transformation|GetActorLocation) "None")))

(fn ConstructionScript
  (|CallParentFunction))