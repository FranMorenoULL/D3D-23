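; BP_Door is a blockout sliding double door that a button trigger sets in motion.
; On BeginPlay it binds to its ButtonReceiver's triggered event, which plays the DoorsLocation timeline.
; The timeline's single AbsoluteYLocation track drives both panels' relative Y in opposite directions, keeping X and Z unchanged.
; The timeline only plays forward, with no reverse or closing logic.
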(event Custom|OnButtonReceiverTriggered
  (bind _doorleft (Variables|Default|GetDoorLeft))
  (bind _doorright (Variables|Default|GetDoorRight))
  (bind _relativelocation (Variables|/Script/Engine.SceneComponent|GetRelativeLocation _doorright))
  (bind _relativelocation_2 (Variables|/Script/Engine.SceneComponent|GetRelativeLocation _doorleft))
  (bind _absolute_y_location (Timeline|Doors%20Location Play)
    (:Update
      (Transformation|SetRelativeLocation _doorleft (Math|Vector|MakeVector (.x _relativelocation_2) (- 0.0 _absolute_y_location) (.z _relativelocation_2)) false false)
      (Transformation|SetRelativeLocation _doorright (Math|Vector|MakeVector (.x _relativelocation) _absolute_y_location (.z _relativelocation)) false false))))

(event EventBeginPlay
  (EventDispatchers|AssignOnButtonReceiverTriggered (Variables|Default|GetButtonReceiver) (delegate Custom|OnButtonReceiverTriggered)))

(fn ConstructionScript)